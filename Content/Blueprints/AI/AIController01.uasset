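; AI controller for a sedan opponent that holds full throttle after a start signal until the car finishes.
; SetData possesses the sedan, then binds its finished event and the HUD's red-light possible-start event.
; The start signal waits a delay, then opens a Tick-driven gate feeding throttle input; finishing closes it.
; On construction, it registers itself in one of two GameInstance AI controller slots.
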(event Custom|CustomEvent_0
  (Utilities|FlowControl|Delay (Variables|Default|GetDelay))
  (CallFunction|PressThrottle))

(event Custom|CustomEvent_1)

(event Custom|PressThrottle
  (Utilities|FlowControl|Gate true) ; enters at Open
)

(event Custom|Release_Throttle
  (Utilities|FlowControl|Gate true) ; enters at Close
)

(event Custom|SetData
  (params (Sedan :type Sedan%20Object%20Reference))
  (bind _output_get (Variables|Default|SetPawnSedan Sedan))
  (Pawn|Possess _output_get)
  (EventDispatchers|BindEventtoFinished _output_get (delegate Custom|Release_Throttle))
  (EventDispatchers|BindEventtoRedlightingPossibleStart (Variables|/Game/Blueprints/Game/GameInstance01.GameInstance01_C|GetHUD (Variables|Default|GetGameInstance)) (delegate Custom|CustomEvent_0))
  (EventDispatchers|BindEventtoFirstTouchbyPlayer (Variables|Default|GetLevelLogic) (delegate Custom|CustomEvent_1)))

(event EventBeginPlay)

(event EventTick
  (params (DeltaSeconds :type Float%20%28single-precision%29))
  (Utilities|FlowControl|Gate true
    (:Exit
      (Default|ThrottleInput01 (Variables|Default|GetPawnSedan) 1.0))))

(fn ConstructionScript
  (Variables|Default|SetGameInstance (CallFunction|GetGameInstance01))
  (Variables|Default|SetLevelLogic (Variables|/Game/Blueprints/Game/GameInstance01.GameInstance01_C|GetLevelLogic (Variables|Default|GetGameInstance)))
  (Utilities|IsValid (Variables|/Game/Blueprints/Game/GameInstance01.GameInstance01_C|GetAIController01 (Variables|Default|GetGameInstance))
    (:Is%20Valid
      (Variables|/Game/Blueprints/Game/GameInstance01.GameInstance01_C|SetAIController02 (Variables|Default|GetGameInstance) self))
    (:Is%20Not%20Valid
      (Variables|/Game/Blueprints/Game/GameInstance01.GameInstance01_C|SetAIController01 (Variables|Default|GetGameInstance) self))))