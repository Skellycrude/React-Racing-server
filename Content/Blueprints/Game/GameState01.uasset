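; Game State for a multiplayer staged-start race that drives the start lights.
; PawnStaged counts staged pawns and compares the count to the game mode's player count minus one.
; On a match it waits briefly, then fires the amber-and-green light event.
; That event and a per-lane red light event, both named as multicasts, forward to LevelLogic on the game instance.
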(event Custom|LightAmberAndGreen_Multi
  ;[1 1 1] LightAmberAndGreenMulti
  (Default|LightAmbersandGreen (Variables|/Game/Blueprints/Game/GameInstance01.GameInstance01_C|GetLevelLogic (CallFunction|GetGameInstance01))))

(event Custom|LightRed_Multi
  (params (Lane :type Integer))
  ;[1 1 1] LightRedMulti
  (Default|LightRed (Variables|/Game/Blueprints/Game/GameInstance01.GameInstance01_C|GetLevelLogic (CallFunction|GetGameInstance01)) Lane))

(event Custom|PawnStaged
  ;[1 1 1] PawnStaged
  (bind _result (Math|Integer|IncrementInt (Variables|State|GetPawnsStaged))
    (:%20%20
      (bind _asmultiplayer_game_mode (Utilities|Casting|CastToMultiplayerGameMode (Game|GetGameMode)))
      (bind _returnvalue (Class|GameModeBase|GetNumPlayers _asmultiplayer_game_mode))
      (if (== (- _returnvalue 1) _result)
        (Utilities|FlowControl|Delay 2.0)
        (CallFunction|LightAmberandGreenMulti)))))

(event EventBeginPlay
  (|CallParentFunction) ; This node is disabled and will not be called.\nDrag off pins to build functionality.
)

(event EventTick
  (params (DeltaSeconds :type Float%20%28single-precision%29))
  (|CallParentFunction DeltaSeconds) ; This node is disabled and will not be called.\nDrag off pins to build functionality.
)

(fn ConstructionScript
  (|CallParentFunction))