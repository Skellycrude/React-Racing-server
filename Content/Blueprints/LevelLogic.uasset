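; Level logic actor for a car race (apparently drag racing) that sets up single or multiplayer sessions, registering itself with the GameInstance on construction.
; Single player spawns player and AI Sedans, builds the HUD and starts the race after the first gas press; multiplayer waits for pawn spawns.
; Routes finish, centerline and redlight events to handlers.
; Reads points via PlayFab and awards them through Cloud Script, updating HUD and local total.
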(event Custom|CustomEvent_0
  (Utilities|FlowControl|DoOnce false
    (:Completed
      (Default|CallFirstTouchbyPlayer)
      (Utilities|FlowControl|Delay 5.0)
      (CallFunction|StartRace (Variables|Default|GetGameInstance) (Variables|Default|GetHUD)))))

(event Custom|ResetFirstTouchByPlayer
  (Utilities|FlowControl|DoOnce false) ; enters at Reset
)

(event Custom|CustomEvent_2
  (params (error :type Play%20Fab%20Error%20Structure) (customData :type Object%20Object%20Reference))
  ;[1 1 1] Get player stats
  (Development|PrintString "Couldn't get player stats"))

(event Custom|GivePoints
  (params (Place :type Integer) (Won3_InHeat :type Boolean))
  ;[1 1 1] Give points
  (Variables|Default|SetPlace Place)
  (Variables|Default|SetWon3_InHeat Won3_InHeat)
  (bind _output_get (Variables|Default|SetPlayFabJsonObject (Class|PlayFabJsonObject|ConstructJsonObject)))
  (Class|PlayFabJsonObject|SetBoolField _output_get "disqualified" (Variables|/Game/Blueprints/Game/GameInstance01.GameInstance01_C|GetDisqualified (Variables|Default|GetGameInstance)))
  (Class|PlayFabJsonObject|SetNumberField (Variables|Default|GetPlayFabJsonObject) "place" (Math|Conversions|ToFloat(Integer) (Variables|Default|GetPlace)))
  (Class|PlayFabJsonObject|SetBoolField (Variables|Default|GetPlayFabJsonObject) "won3InHeat" (Variables|Default|GetWon3_InHeat))
  (|ExecuteCloudScript (Utilities|Struct|MakeClientExecuteCloudScriptRequest "givePoints" (Variables|Default|GetPlayFabJsonObject) false "pfenum_Live" 0) (delegate Custom|CustomEvent_7) (delegate Custom|CustomEvent_8)))

(event Custom|CustomEvent_3
  (params (result :type Client%20Get%20Player%20Statistics%20Result%20Structure) (customData :type Object%20Object%20Reference))
  ;[1 1 1] Get player stats
  (Variables|/Game/Blueprints/Game/GameInstance01.GameInstance01_C|SetPoints (Variables|Default|GetGameInstance) (Math|Float|Truncate (Class|PlayFabJsonObject|GetNumberField (Utilities|Array|Get(acopy) (.statistics result)) "Value"))))

(event Custom|GetPlayerStats
  ;[1 1 1] Get player stats
  (|GetPlayerStatisticVersions (Utilities|Struct|MakeClientGetPlayerStatisticVersionsRequest "Points") (delegate Custom|CustomEvent_1) (delegate Custom|CustomEvent_2)))

(event Custom|CustomEvent_4
  (params (error :type Play%20Fab%20Error%20Structure) (customData :type Object%20Object%20Reference))
  ;[1 1 1] Get player stats
)

(event Custom|CustomEvent_7
  (params (result :type Client%20Execute%20Cloud%20Script%20Result%20Structure) (customData :type Object%20Object%20Reference))
  (bind _returnvalue (Class|PlayFabJsonObject|GetObjectField (.functionresult result) "points"))
  ;[1 1 1] Update HUD and local points
  (Variables|Default|SetPlayFabJsonObject _returnvalue)
  (Default|FinishMessage (Variables|/Game/Blueprints/Game/GameInstance01.GameInstance01_C|GetHUD (Variables|Default|GetGameInstance)) (Math|Float|Truncate (Class|PlayFabJsonObject|GetNumberField _returnvalue "pointsGiven")) (Variables|Default|GetPlace) (Class|PlayFabJsonObject|GetBoolField _returnvalue "receivedBonusPoints") (Math|Float|Truncate (Class|PlayFabJsonObject|GetNumberField _returnvalue "bonusPointsGiven")))
  (Variables|/Game/Blueprints/Game/GameInstance01.GameInstance01_C|SetPoints (Variables|Default|GetGameInstance) (Math|Float|Truncate (Class|PlayFabJsonObject|GetNumberField (Variables|Default|GetPlayFabJsonObject) "newTotalPoints"))))

(event Custom|CustomEvent_5
  (params (Pawn :type Sedan%20Object%20Reference))
  (switch Utilities|FlowControl|Switch|SwitchonGameMode (CallFunction|SingleorMultiplayer)
    (:NewEnumerator1
      (Utilities|FlowControl|Delay 5.0)
      (Default|CallCountdownStart (Variables|Default|GetGameInstance)))
    (:NewEnumerator2
      (CallFunction|GetPlayerStats)
      (CallFunction|CreateHUD (Variables|Default|GetGameInstance)))))

(event Custom|CustomEvent_8
  (params (error :type Play%20Fab%20Error%20Structure) (customData :type Object%20Object%20Reference))
  ;[1 1 1] Give points
  (Development|PrintString "Couldn't give points"))

(event Custom|CustomEvent_1
  (params (result :type Client%20Get%20Player%20Statistic%20Versions%20Result%20Structure) (customData :type Object%20Object%20Reference))
  ;[1 1 1] Get player stats
  (|GetPlayerStatistics (Utilities|Struct|MakeClientGetPlayerStatisticsRequest "Points" (.statisticversions result)) (delegate Custom|CustomEvent_3) (delegate Custom|CustomEvent_4)))

(event EventBeginPlay
  (bind _gameinstance (Variables|Default|GetGameInstance))
  (bind _gameinstance_2 (Variables|Default|GetGameInstance))
  (bind _aicontroller02 (Variables|/Game/Blueprints/Game/GameInstance01.GameInstance01_C|GetAIController02 _gameinstance_2))
  (switch Utilities|FlowControl|Switch|SwitchonGameMode (CallFunction|SingleorMultiplayer)
    (:NewEnumerator0
      (CallFunction|GetPlayerStats)
      (Game|SpawnActorfromClass "/Game/VehicleBP/Sedan/Sedan.Sedan_C" (Math|Transform|MakeTransform (Transformation|GetActorLocation (Utilities|Array|Get(acopy) (Variables|Default|GetPlayerStarts))) "0,-90.000000, 0") "AlwaysSpawn" 0 true 0)
      (bind _returnvalue (Game|SpawnActorfromClass "/Game/Blueprints/AI/AIController01.AIController01_C" (Math|Transform|MakeTransform "0, 0, 0") "Undefined" 0 0))
      (Game|SpawnActorfromClass "/Game/VehicleBP/Sedan/Sedan.Sedan_C" (Math|Transform|MakeTransform (Transformation|GetActorLocation (Utilities|Array|Get(acopy) (Variables|Default|GetPlayerStarts) 1)) "0,-90.000000, 0") "AlwaysSpawn" _returnvalue false 0)
      (switch int (Variables|/Game/Blueprints/Game/GameInstance01.GameInstance01_C|GetNumberOfRacers (Variables|Default|GetGameInstance))
        (:Default
          _)
        (:3
          (bind _returnvalue_2 (Game|SpawnActorfromClass "/Game/Blueprints/AI/AIController01.AIController01_C" (Math|Transform|MakeTransform "0, 0, 0") "AlwaysSpawn" 0 0))
          (Game|SpawnActorfromClass "/Game/VehicleBP/Sedan/Sedan.Sedan_C" (Math|Transform|MakeTransform (Transformation|GetActorLocation (Utilities|Array|Get(acopy) (Variables|Default|GetPlayerStarts) 2)) "0,-90.000000, 0") "AlwaysSpawn" _returnvalue_2 false 0)))
      (bind (_hud01 _touchinterface01) (CallFunction|CreateHUD (Variables|Default|GetGameInstance)))
      (Variables|Default|SetHUD _hud01)
      (bind _output_get (Variables|Default|SetTouchInterface01 _touchinterface01))
      (Variables|Default|SetGasPedal (Variables|/Game/UI/TouchInterface01.TouchInterface01_C|GetGasPedal _output_get))
      (EventDispatchers|BindEventtoGasButtonPressed (Variables|Default|GetGasPedal) (delegate Custom|CustomEvent_0))
      (bind _asplayer_controller_single_player (Utilities|Casting|CastToPlayerControllerSinglePlayer (Game|GetPlayerController 0)))
      (Default|SetData _asplayer_controller_single_player (Variables|/Game/Blueprints/Game/GameInstance01.GameInstance01_C|GetPlayerPawn (Variables|Default|GetGameInstance)))
      (Default|SetData (Variables|/Game/Blueprints/Game/GameInstance01.GameInstance01_C|GetAIController01 _gameinstance) (Variables|/Game/Blueprints/Game/GameInstance01.GameInstance01_C|GetAIPawn01 _gameinstance))
      (Utilities|IsValid _aicontroller02
        (:Is%20Valid
          (Default|SetData _aicontroller02 (Variables|/Game/Blueprints/Game/GameInstance01.GameInstance01_C|GetAIPawn02 _gameinstance_2)))
        (:Is%20Not%20Valid
          _))
      (CallFunction|GetReadyforRace (Variables|Default|GetGameInstance) (Variables|Default|GetHUD)))
    (:NewEnumerator1
      (EventDispatchers|BindEventtoPlayerPawnSpawned (Variables|Default|GetGameInstance) (delegate Custom|CustomEvent_5) :!label _label))
    (:NewEnumerator2
      (goto _label))))

(event Collision|EventActorBeginOverlap
  (params (OtherActor :type Actor%20Object%20Reference)))

(event EventTick
  (params (DeltaSeconds :type Float%20%28single-precision%29)))

(fn ConstructionScript
  (bind _output_get (Variables|Default|SetGameInstance (CallFunction|GetGameInstance)))
  (Variables|Default|SetPlayerStarts (Variables|/Game/Blueprints/Game/GameInstance01.GameInstance01_C|GetPlayerStarts _output_get))
  (CallFunction|SetLevelLogic (Variables|Default|GetGameInstance) self))

(fn PawnFinished
  (params (Pawn :type Sedan%20Object%20Reference))
  (bind _gameinstance (Variables|Default|GetGameInstance))
  (switch Utilities|FlowControl|Switch|SwitchonGameMode (CallFunction|SingleorMultiplayer)
    (:NewEnumerator0
      (if (== Pawn (Variables|/Game/Blueprints/Game/GameInstance01.GameInstance01_C|GetPlayerPawn (Variables|Default|GetGameInstance)))
        (CallFunction|PlayerFinished _gameinstance (Variables|/Game/Blueprints/Game/GameInstance01.GameInstance01_C|GetHUD _gameinstance) :!label _label)
        (else
          (CallFunction|AIFinished (Variables|Default|GetGameInstance)))))
    (:NewEnumerator2
      (goto _label))))

(fn PawnCrossedCenterline
  (params (Pawn :type Sedan%20Object%20Reference))
  (if (== Pawn (Variables|/Game/Blueprints/Game/GameInstance01.GameInstance01_C|GetPlayerPawn (Variables|Default|GetGameInstance)))
    (CallFunction|PlayerCrossedCenterline (Variables|Default|GetGameInstance))))

(fn PawnRedlighted
  (params (Pawn :type Sedan%20Object%20Reference))
  (if (== Pawn (Variables|/Game/Blueprints/Game/GameInstance01.GameInstance01_C|GetPlayerPawn (Variables|Default|GetGameInstance)))
    (CallFunction|PlayerRedlighted (Variables|Default|GetGameInstance))))