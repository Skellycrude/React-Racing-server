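; Single-player controller that possesses the player's vehicle and drives its throttle from the touch gas pedal.
; It registers itself with the GameInstance, then SetData binds pedal press/release and LevelLogic's first-touch event, which releases the handbrake and enables throttle.
; Tick applies full or zero throttle in Race mode.
; Burnout mode also heats or cools tire temperature, updating throttle only until the temperature reaches its limit.
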(event Custom|ThrottlePressed
  (Variables|Default|SetbThrottlePressed true))

(event Custom|ThrottleReleased
  (Variables|Default|SetbThrottlePressed false))

(event Custom|CustomEvent_0
  (Class|WheeledVehicleMovementComponent|SetHandbrakeInput (Variables|/Script/PhysXVehicles.WheeledVehicle|GetVehicleMovement (Variables|Default|GetPawn01)) false)
  (Default|EnableThrottle (Variables|Default|GetPawn01)))

(event Custom|CustomEvent_1
  (CallFunction|ThrottlePressed))

(event Custom|CustomEvent_2
  (CallFunction|ThrottleReleased))

(event Custom|SetData
  (params (Pawn :type Sedan%20Object%20Reference))
  (bind _output_get (Variables|Default|SetPawn01 Pawn))
  (Pawn|Possess _output_get)
  (Variables|Default|SetTouchInterface01 (Variables|/Game/Blueprints/Game/GameInstance01.GameInstance01_C|GetTouchInterface01 (Variables|Default|GetGameInstance)))
  (Variables|Default|SetGasPedal (Variables|/Game/UI/TouchInterface01.TouchInterface01_C|GetGasPedal (Variables|/Game/Blueprints/Game/GameInstance01.GameInstance01_C|GetTouchInterface01 (Variables|Default|GetGameInstance))))
  (Variables|Default|SetLevelLogic (Variables|/Game/Blueprints/Game/GameInstance01.GameInstance01_C|GetLevelLogic (Variables|Default|GetGameInstance)))
  (EventDispatchers|BindEventtoGasButtonPressed (Variables|Default|GetGasPedal) (delegate Custom|CustomEvent_1))
  (EventDispatchers|BindEventtoGasButtonReleased (Variables|Default|GetGasPedal) (delegate Custom|CustomEvent_2))
  (EventDispatchers|BindEventtoFirstTouchbyPlayer (Variables|Default|GetLevelLogic) (delegate Custom|CustomEvent_0)))

(event EventBeginPlay)

(event EventTick
  (params (DeltaSeconds :type Float%20%28single-precision%29))
  (bind _pawn01 (Variables|Default|GetPawn01))
  (bind _pawn01_2 (Variables|Default|GetPawn01))
  (if (Variables|Default|GetbThrottlePressed)
    (switch Utilities|FlowControl|Switch|SwitchonVehicleMode (Variables|Default|GetVehicleMode)
      (:NewEnumerator0
        (Default|ThrottleInput01 (Variables|Default|GetPawn01) 1.0 :!label _label))
      (:NewEnumerator1
        (if (not (>= (Variables|/Game/VehicleBP/Sedan/Sedan.Sedan_C|GetTireTemp (Variables|Default|GetPawn01)) 125.0))
          (Variables|/Game/VehicleBP/Sedan/Sedan.Sedan_C|SetTireTemp _pawn01 (+ (Variables|/Game/VehicleBP/Sedan/Sedan.Sedan_C|GetTireTemp _pawn01) (* DeltaSeconds 1e+02)))
          (goto _label))))
    (else
      (switch Utilities|FlowControl|Switch|SwitchonVehicleMode (Variables|Default|GetVehicleMode)
        (:NewEnumerator0
          (Default|ThrottleInput01 (Variables|Default|GetPawn01) 0.0 :!label _label_2))
        (:NewEnumerator1
          (if (not (<= (Variables|/Game/VehicleBP/Sedan/Sedan.Sedan_C|GetTireTemp (Variables|Default|GetPawn01)) 0.0))
            (Variables|/Game/VehicleBP/Sedan/Sedan.Sedan_C|SetTireTemp _pawn01_2 (- (Variables|/Game/VehicleBP/Sedan/Sedan.Sedan_C|GetTireTemp _pawn01_2) (* 7e+01 DeltaSeconds)))
            (goto _label_2)))))))

(fn ConstructionScript
  (bind _output_get (Variables|Default|SetGameInstance (CallFunction|GetGameInstance)))
  (Variables|/Game/Blueprints/Game/GameInstance01.GameInstance01_C|SetPlayerControllerSinglePlayer _output_get self))