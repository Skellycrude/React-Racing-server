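; Multiplayer player controller for a car racing game with Race and Burnout vehicle modes.
; On authority it spawns and possesses a Sedan at the first valid player start, clears that slot and binds the race countdown.
; Remote local controllers bind gas-pedal events to a throttle flag, which Tick turns into throttle input, ramping tire temperature during Burnout.
; Further events enable or stop the vehicle and update the matchmaking HUD.
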(event Custom|ThrottlePressed
  (Variables|Default|SetbThrottlePressed true))

(event Custom|StopVehicle
  (CallFunction|CloseInput)
  (CallFunction|StopVehicle (Variables|Default|GetPawn01)))

(event Custom|CountdownStart
  (bind _gameinstance (Variables|Default|GetGameInstance))
  (CallFunction|StartRace _gameinstance (Variables|/Game/Blueprints/Game/GameInstance01.GameInstance01_C|GetHUD _gameinstance)))

(event Custom|ThrottleReleased
  (Variables|Default|SetbThrottlePressed false))

(event Custom|CloseInput
  (Utilities|FlowControl|Gate false) ; enters at Close
)

(event Custom|CustomEvent_0
  (CallFunction|ThrottlePressed))

(event Custom|CustomEvent_1
  (CallFunction|ThrottleReleased))

(event Custom|OnMathcmakingMatchStarting
  (params (PlayerCount :type Integer))
  (bind _hudreference (Variables|Default|GetHUDReference))
  (bind _matchmakinginvite (Variables|/Matchmaking/UI/BPW_MatchmakingHUD.BPW_MatchmakingHUD_C|GetMatchmakingInvite _hudreference))
  (Default|NoDialogShow _matchmakinginvite)
  (Default|ReadyProgressUpdate _matchmakinginvite PlayerCount)
  (Variables|Default|SetMatchmaking_IsQueued false)
  (Class|BPIMatchmakingPlayerController|MatchmakingHUDPlayerIsReady(Message) self)
  (Variables|/Matchmaking/UI/BPW_Matchmaking_Invite.BPW_Matchmaking_Invite_C|SetIsReady _matchmakinginvite true))

(event Custom|EnableMovement
  (Class|WheeledVehicleMovementComponent|SetHandbrakeInput (Variables|/Script/PhysXVehicles.WheeledVehicle|GetVehicleMovement (Variables|Default|GetPawn01)) false)
  (Default|EnableThrottle (Variables|Default|GetPawn01))
  (CallFunction|OpenInput))

(event Custom|CustomEvent_2
  (bind _gameinstance (Variables|Default|GetGameInstance))
  (bind _gaspedal (Variables|/Game/Blueprints/Game/GameInstance01.GameInstance01_C|GetGasPedal _gameinstance))
  (EventDispatchers|BindEventtoGasButtonPressed _gaspedal (delegate Custom|CustomEvent_0))
  (EventDispatchers|BindEventtoGasButtonReleased _gaspedal (delegate Custom|CustomEvent_1)))

(event Custom|OpenInput
  (Utilities|FlowControl|Gate false) ; enters at Open
)

(event Custom|CustomEvent_3
  (CallFunction|CountdownStart))

(event EventBeginPlay
  (bind _gameinstance (Variables|Default|GetGameInstance))
  (bind _playerstarts (Variables|/Game/Blueprints/Game/GameInstance01.GameInstance01_C|GetPlayerStarts _gameinstance))
  (|CallParentFunction)
  (Networking|SwitchHasAuthority
    (:Authority
      (bind (_array_element _array_index) (Utilities|Array|ForEachLoopwithBreak _playerstarts :!label _label)
        (:LoopBody
          (Utilities|IsValid _array_element
            (:Is%20Valid
              (bind _returnvalue (Game|SpawnActorfromClass "/Game/VehicleBP/Sedan/Sedan.Sedan_C" (Math|Transform|MakeTransform (Transformation|GetActorLocation _array_element) "0,-90.000000, 0") "AlwaysSpawn" 0 false 0))
              (Pawn|Possess _returnvalue)
              (Variables|Default|SetPawn01 _returnvalue)
              (Utilities|Array|SetArrayElem _playerstarts _array_index 0)
              (goto _label Break))))
        (:Completed
          (EventDispatchers|BindEventtoCountdownStart (Variables|Default|GetGameInstance) (delegate Custom|CustomEvent_3)))))
    (:Remote
      (if (Pawn|IsLocalPlayerController self)
        (EventDispatchers|BindEventtoGasPedalCreated (Variables|Default|GetGameInstance) (delegate Custom|CustomEvent_2))))))

(event EventMatchmakingMatchStarting
  (params (PlayerCounter :type Integer))
  (CallFunction|OnMathcmakingMatchStarting PlayerCounter))

(event EventTick
  (params (DeltaSeconds :type Float%20%28single-precision%29))
  (bind _pawn01 (Variables|Default|GetPawn01))
  (bind _pawn01_2 (Variables|Default|GetPawn01))
  (if (Variables|Default|GetbThrottlePressed)
    (switch Utilities|FlowControl|Switch|SwitchonVehicleMode (Variables|Default|GetVehicleMode)
      (:NewEnumerator0
        (Default|ThrottleInput01 (Variables|Default|GetPawn01) 1.0 :!label _label))
      (:NewEnumerator1
        (if (not (>= (Variables|/Game/VehicleBP/Sedan/Sedan.Sedan_C|GetTireTemp (Variables|Default|GetPawn01)) 125.0))
          (Variables|/Game/VehicleBP/Sedan/Sedan.Sedan_C|SetTireTemp _pawn01 (+ (Variables|/Game/VehicleBP/Sedan/Sedan.Sedan_C|GetTireTemp _pawn01) (* DeltaSeconds 1e+02)))
          (goto _label))))
    (else
      (switch Utilities|FlowControl|Switch|SwitchonVehicleMode (Variables|Default|GetVehicleMode)
        (:NewEnumerator0
          (Default|ThrottleInput01 (Variables|Default|GetPawn01) 0.0 :!label _label_2))
        (:NewEnumerator1
          (if (not (<= (Variables|/Game/VehicleBP/Sedan/Sedan.Sedan_C|GetTireTemp (Variables|Default|GetPawn01)) 0.0))
            (Variables|/Game/VehicleBP/Sedan/Sedan.Sedan_C|SetTireTemp _pawn01_2 (- (Variables|/Game/VehicleBP/Sedan/Sedan.Sedan_C|GetTireTemp _pawn01_2) (* 7e+01 DeltaSeconds)))
            (goto _label_2)))))))

(fn ConstructionScript
  (|CallParentFunction)
  (Variables|Default|SetGameInstance (CallFunction|GetGameInstance)))