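; Shared function library for a drag racing game, covering race setup, start, finish, disqualification, HUD creation and PlayFab setup.
; GameInstance01 holds the shared state: pawns, start points, finish order and heat progress, reset between races as vehicles are stopped and teleported back.
; PlayerFinished derives place from finish order and passes heat wins to LevelLogic for scoring, leaving local GivePoints unused.
; SingleOrMultiplayer treats a missing GameMode as a client.
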(fn SetData
  (params (GameInstance :type Game%20Instance%20Object%20Reference%20%28by%20ref%29) (PlayerStart1 :type Player%20Start%20Object%20Reference) (PlayerStart2 :type Player%20Start%20Object%20Reference) (PlayerStart3 :type Player%20Start%20Object%20Reference) (ChristmasTree :type Static%20Mesh%20Actor%20Object%20Reference))
  (bind _asgame_instance_01 (Utilities|Casting|CastToGameInstance01 GameInstance))
  (LocalVariables|SetGameInstanceLocal _asgame_instance_01)
  (LocalVariables|SetPlayerStart1Local PlayerStart1)
  (LocalVariables|SetPlayerStart2Local PlayerStart2)
  (LocalVariables|SetPlayerStart3Local PlayerStart3)
  (Variables|/Game/Blueprints/Game/GameInstance01.GameInstance01_C|SetChristmasTree (LocalVariables|GetGameInstanceLocal) ChristmasTree)
  (Utilities|Array|Clear (Variables|/Game/Blueprints/Game/GameInstance01.GameInstance01_C|GetPlayerStarts (LocalVariables|GetGameInstanceLocal)))
  (Utilities|Array|Add (Variables|/Game/Blueprints/Game/GameInstance01.GameInstance01_C|GetPlayerStarts (LocalVariables|GetGameInstanceLocal)) (LocalVariables|GetPlayerStart1Local))
  (Utilities|Array|Add (Variables|/Game/Blueprints/Game/GameInstance01.GameInstance01_C|GetPlayerStarts (LocalVariables|GetGameInstanceLocal)) (LocalVariables|GetPlayerStart2Local))
  (Utilities|Array|Add (Variables|/Game/Blueprints/Game/GameInstance01.GameInstance01_C|GetPlayerStarts (LocalVariables|GetGameInstanceLocal)) (LocalVariables|GetPlayerStart3Local)))

(fn CreateHUD
  (LocalVariables|SetGameInstanceLocal (CallFunction|GetGameInstance))
  (bind _returnvalue (UserInterface|CreateWidget "/Game/UI/HUD01.HUD01_C"))
  (bind _output_get (LocalVariables|SetHUD01Local _returnvalue))
  (Variables|/Game/Blueprints/Game/GameInstance01.GameInstance01_C|SetHUD (LocalVariables|GetGameInstanceLocal) _output_get)
  (bind _returnvalue_2 (UserInterface|CreateWidget "/Game/UI/TouchInterface01.TouchInterface01_C" (Game|GetPlayerController 0)))
  (bind _output_get_2 (LocalVariables|SetTouchInterface01Local _returnvalue_2))
  (Variables|/Game/Blueprints/Game/GameInstance01.GameInstance01_C|SetTouchInterface01 (LocalVariables|GetGameInstanceLocal) _output_get_2)
  (UserInterface|Viewport|AddtoViewport (LocalVariables|GetHUD01Local) 0)
  (UserInterface|Viewport|AddtoViewport (LocalVariables|GetTouchInterface01Local) 0)
  (Default|CallHUDCreated (LocalVariables|GetGameInstanceLocal))
  (return (LocalVariables|GetHUD01Local) (LocalVariables|GetTouchInterface01Local)))

(fn SetLevelLogic
  (params (GameInstance :type Game%20Instance%20Object%20Reference%20%28by%20ref%29) (LevelLogic :type Level%20Logic%20Object%20Reference))
  (bind _asgame_instance_01 (Utilities|Casting|CastToGameInstance01 GameInstance))
  (Variables|/Game/Blueprints/Game/GameInstance01.GameInstance01_C|SetLevelLogic _asgame_instance_01 LevelLogic))

(fn AIFinished
  (params (GameInstance :type Game%20Instance%20Object%20Reference%20%28by%20ref%29))
  (bind _asgame_instance_01 (Utilities|Casting|CastToGameInstance01 GameInstance))
  (Utilities|Array|Add (Variables|/Game/Blueprints/Game/GameInstance01.GameInstance01_C|GetFinishOrder _asgame_instance_01) 0)
  (Variables|/Game/Blueprints/Game/GameInstance01.GameInstance01_C|SetFinishOrder _asgame_instance_01 (Variables|/Game/Blueprints/Game/GameInstance01.GameInstance01_C|GetFinishOrder _asgame_instance_01)))

(fn PlayerFinished
  (params (GameInstance :type Game%20Instance%20Object%20Reference%20%28by%20ref%29) (HUD :type HUD01%20Object%20Reference%20%28by%20ref%29))
  (LocalVariables|SetHUDLocal HUD)
  (bind _asgame_instance_01 (Utilities|Casting|CastToGameInstance01 GameInstance))
  (LocalVariables|SetGameInstanceLocal _asgame_instance_01)
  (LocalVariables|SetPlaceLocal (Utilities|Array|Length (Variables|/Game/Blueprints/Game/GameInstance01.GameInstance01_C|GetFinishOrder (LocalVariables|GetGameInstanceLocal))))
  (bind _won3_inheat (CallFunction|UpdateRacesWoninHeat (LocalVariables|GetGameInstanceLocal) (LocalVariables|GetPlaceLocal)))
  (Default|GivePoints (Variables|/Game/Blueprints/Game/GameInstance01.GameInstance01_C|GetLevelLogic (LocalVariables|GetGameInstanceLocal)) (LocalVariables|GetPlaceLocal) _won3_inheat))

(fn PlayerDisqualified
  (params (GameInstance :type Game%20Instance%20Object%20Reference%20%28by%20ref%29))
  (bind _asgame_instance_01 (Utilities|Casting|CastToGameInstance01 GameInstance))
  (Variables|/Game/Blueprints/Game/GameInstance01.GameInstance01_C|SetDisqualified _asgame_instance_01 true))

(fn PlayerCrossedCenterline
  (params (GameInstance :type Game%20Instance%20Object%20Reference%20%28by%20ref%29))
  (CallFunction|PlayerDisqualified GameInstance))

(fn PlayerRedlighted
  (params (GameInstance :type Game%20Instance%20Object%20Reference%20%28by%20ref%29))
  (CallFunction|PlayerDisqualified GameInstance))

(fn GivePoints
  (params (GameInstance :type Game%20Instance%20Object%20Reference%20%28by%20ref%29) (Place :type Integer))
  (bind _pointsforwin (LocalVariables|GetPointsForWin))
  (bind _pointsforloss (LocalVariables|GetPointsForLoss))
  (LocalVariables|SetPlaceLocal Place)
  (bind _asgame_instance_01 (Utilities|Casting|CastToGameInstance01 GameInstance))
  (bind _output_get (LocalVariables|SetGameInstanceLocal _asgame_instance_01))
  (LocalVariables|SetPointsOriginal (Variables|/Game/Blueprints/Game/GameInstance01.GameInstance01_C|GetPoints _output_get))
  (LocalVariables|SetSaveGameLocal (Variables|/Game/Blueprints/Game/GameInstance01.GameInstance01_C|GetSaveGame (LocalVariables|GetGameInstanceLocal)))
  (LocalVariables|SetRacesWonInHeatLocal (Variables|/Game/Blueprints/Game/GameInstance01.GameInstance01_C|GetRacesWonInHeat (LocalVariables|GetGameInstanceLocal)))
  (if (Variables|/Game/Blueprints/Game/GameInstance01.GameInstance01_C|GetDisqualified (LocalVariables|GetGameInstanceLocal))
    (LocalVariables|SetPointsGivenLocal _pointsforloss :!label _label)
    (bind _output_get_2 (Variables|/Game/Blueprints/Game/GameInstance01.GameInstance01_C|SetPoints (LocalVariables|GetGameInstanceLocal) (+ (LocalVariables|GetPointsOriginal) _pointsforloss)))
    (Variables|/Game/Blueprints/SaveGame01.SaveGame01_C|SetPoints (LocalVariables|GetSaveGameLocal) _output_get_2)
    (SaveGame|SaveGametoSlot (LocalVariables|GetSaveGameLocal) "Save01")
    (else
      (switch int (LocalVariables|GetPlaceLocal)
        (:0
          (bind _output_get_3 (LocalVariables|SetRacesWonInHeatLocal (+ (LocalVariables|GetRacesWonInHeatLocal) 1)))
          (Variables|/Game/Blueprints/Game/GameInstance01.GameInstance01_C|SetRacesWonInHeat (LocalVariables|GetGameInstanceLocal) _output_get_3)
          (if (== (LocalVariables|GetRacesWonInHeatLocal) 3)
            (LocalVariables|SetWon3InHeatLocal true)
            (LocalVariables|SetBonusPointsLocal (Variables|/Game/Blueprints/Game/GameInstance01.GameInstance01_C|GetBonusPointsFor3Wins (LocalVariables|GetGameInstanceLocal))))
          (LocalVariables|SetPointsGivenLocal _pointsforwin)
          (bind _output_get_4 (Variables|/Game/Blueprints/Game/GameInstance01.GameInstance01_C|SetPoints (LocalVariables|GetGameInstanceLocal) (+ (LocalVariables|GetPointsOriginal) _pointsforwin (LocalVariables|GetBonusPointsLocal))))
          (Variables|/Game/Blueprints/SaveGame01.SaveGame01_C|SetPoints (LocalVariables|GetSaveGameLocal) _output_get_4)
          (SaveGame|SaveGametoSlot (LocalVariables|GetSaveGameLocal) "Save01"))
        (:1
          (goto _label))
        (:2
          (goto _label)))))
  (return (LocalVariables|GetPointsGivenLocal) (LocalVariables|GetWon3InHeatLocal) (LocalVariables|GetBonusPointsLocal)))

(fn StartRace
  (params (GameInstance :type Game%20Instance%20Object%20Reference%20%28by%20ref%29) (HUD :type HUD01%20Object%20Reference))
  (LocalVariables|SetHUDLocal HUD)
  (bind _asgame_instance_01 (Utilities|Casting|CastToGameInstance01 GameInstance))
  (LocalVariables|SetGameInstanceLocal _asgame_instance_01)
  (LocalVariables|SetPlayerPawnLocal (Variables|/Game/Blueprints/Game/GameInstance01.GameInstance01_C|GetPlayerPawn (LocalVariables|GetGameInstanceLocal)))
  (LocalVariables|SetAI01PawnLocal (Variables|/Game/Blueprints/Game/GameInstance01.GameInstance01_C|GetAIPawn01 (LocalVariables|GetGameInstanceLocal)))
  (LocalVariables|SetAI02PawnLocal (Variables|/Game/Blueprints/Game/GameInstance01.GameInstance01_C|GetAIPawn02 (LocalVariables|GetGameInstanceLocal)))
  (switch Utilities|FlowControl|Switch|SwitchonGameMode (CallFunction|SingleorMultiplayer)
    (:NewEnumerator0
      (bind _asplayer_controller_single_player (Utilities|Casting|CastToPlayerControllerSinglePlayer (Pawn|GetController (LocalVariables|GetPlayerPawnLocal))))
      (Variables|/Game/Blueprints/Player/PlayerControllerSinglePlayer.PlayerControllerSinglePlayer_C|SetVehicleMode _asplayer_controller_single_player "NewEnumerator0")
      (Default|EnableThrottle (LocalVariables|GetAI01PawnLocal))
      (Utilities|IsValid (LocalVariables|GetAI02PawnLocal)
        (:Is%20Valid
          (Default|EnableThrottle (LocalVariables|GetAI02PawnLocal)))
        (:Is%20Not%20Valid
          _)))
    (:NewEnumerator2
      (bind _asplayer_controller_multiplayer (Utilities|Casting|CastToPlayerControllerMultiplayer (Pawn|GetController (LocalVariables|GetPlayerPawnLocal))))
      (Variables|/Game/Blueprints/Player/PlayerControllerMultiplayer.PlayerControllerMultiplayer_C|SetVehicleMode _asplayer_controller_multiplayer "NewEnumerator0")))
  (Default|EnableThrottle (LocalVariables|GetPlayerPawnLocal)))

(fn ClearRaceData
  (params (GameInstance :type Game%20Instance%20Object%20Reference%20%28by%20ref%29))
  (bind _asgame_instance_01 (Utilities|Casting|CastToGameInstance01 GameInstance))
  (bind _output_get (LocalVariables|SetGameInstanceLocal _asgame_instance_01))
  (Utilities|Array|Clear (Variables|/Game/Blueprints/Game/GameInstance01.GameInstance01_C|GetFinishOrder _output_get))
  (Variables|/Game/Blueprints/Game/GameInstance01.GameInstance01_C|SetDisqualified (LocalVariables|GetGameInstanceLocal) false)
  (Variables|/Game/Blueprints/Game/GameInstance01.GameInstance01_C|SetPawnsStaged (LocalVariables|GetGameInstanceLocal) 0)
  (Variables|/Game/Blueprints/Game/GameInstance01.GameInstance01_C|SetGreenLightOn (LocalVariables|GetGameInstanceLocal) false)
  (Default|ResetAllLights (Variables|/Game/Blueprints/Game/GameInstance01.GameInstance01_C|GetLevelLogic (LocalVariables|GetGameInstanceLocal))))

(fn StopVehicle
  (params (Pawn :type Sedan%20Object%20Reference))
  (bind _output_get (LocalVariables|SetPawnLocal Pawn))
  (bind _asaicontroller_01 (Utilities|Casting|CastToAIController01 (Pawn|GetController _output_get))
    (:then
      (Default|ReleaseThrottle _asaicontroller_01))
    (:CastFailed
      (Input|DisableInput (LocalVariables|GetPawnLocal) 0)))
  (Class|WheeledVehicleMovementComponent|SetThrottleInput (Variables|/Script/PhysXVehicles.WheeledVehicle|GetVehicleMovement (LocalVariables|GetPawnLocal)) 0.0)
  (Class|WheeledVehicleMovementComponent|SetHandbrakeInput (Variables|/Script/PhysXVehicles.WheeledVehicle|GetVehicleMovement (LocalVariables|GetPawnLocal)) true)
  (Class|PrimitiveComponent|SetAllPhysicsLinearVelocity (Variables|/Script/Engine.MovementComponent|GetUpdatedPrimitive (Variables|/Script/PhysXVehicles.WheeledVehicle|GetVehicleMovement (LocalVariables|GetPawnLocal))) "0, 0, 0" false))

(fn TrackRacesinHeat
  (params (GameInstance :type Game%20Instance%20Object%20Reference%20%28by%20ref%29))
  (bind _asgame_instance_01 (Utilities|Casting|CastToGameInstance01 GameInstance))
  (bind _output_get (LocalVariables|SetGameInstanceLocal _asgame_instance_01))
  (LocalVariables|SetCurrentRaceInHeatLocal (Variables|/Game/Blueprints/Game/GameInstance01.GameInstance01_C|GetCurrentRaceInHeat _output_get))
  (LocalVariables|SetRacesInHeatLocal (Variables|/Game/Blueprints/Game/GameInstance01.GameInstance01_C|GetRacesInHeat (LocalVariables|GetGameInstanceLocal)))
  (if (== (LocalVariables|GetCurrentRaceInHeatLocal) (LocalVariables|GetRacesInHeatLocal))
    (LocalVariables|SetCurrentRaceInHeatLocal 1)
    (Variables|/Game/Blueprints/Game/GameInstance01.GameInstance01_C|SetRacesWonInHeat (LocalVariables|GetGameInstanceLocal) 0)
    (else
      (LocalVariables|SetCurrentRaceInHeatLocal (+ (LocalVariables|GetCurrentRaceInHeatLocal) 1))))
  (Variables|/Game/Blueprints/Game/GameInstance01.GameInstance01_C|SetCurrentRaceInHeat (LocalVariables|GetGameInstanceLocal) (LocalVariables|GetCurrentRaceInHeatLocal)))

(fn GetReadyforRace
  (params (GameInstance :type Game%20Instance%20Object%20Reference%20%28by%20ref%29) (HUD :type HUD01%20Object%20Reference))
  (LocalVariables|SetHUDLocal HUD)
  (bind _asgame_instance_01 (Utilities|Casting|CastToGameInstance01 GameInstance))
  (LocalVariables|SetGameInstanceLocal _asgame_instance_01)
  (LocalVariables|SetPlayerPawnLocal (Variables|/Game/Blueprints/Game/GameInstance01.GameInstance01_C|GetPlayerPawn (LocalVariables|GetGameInstanceLocal)))
  (LocalVariables|SetAIPawn01Local (Variables|/Game/Blueprints/Game/GameInstance01.GameInstance01_C|GetAIPawn01 (LocalVariables|GetGameInstanceLocal)))
  (LocalVariables|SetAIPawn02Local (Variables|/Game/Blueprints/Game/GameInstance01.GameInstance01_C|GetAIPawn02 (LocalVariables|GetGameInstanceLocal)))
  (LocalVariables|SetLevelLogicLocal (Variables|/Game/Blueprints/Game/GameInstance01.GameInstance01_C|GetLevelLogic (LocalVariables|GetGameInstanceLocal)))
  (bind _asplayer_controller_single_player (Utilities|Casting|CastToPlayerControllerSinglePlayer (Pawn|GetController (LocalVariables|GetPlayerPawnLocal))))
  (LocalVariables|SetPlayerControllerSinglePlayerLocal _asplayer_controller_single_player)
  (CallFunction|ClearRaceData (LocalVariables|GetGameInstanceLocal))
  (CallFunction|StopVehicle (LocalVariables|GetPlayerPawnLocal))
  (CallFunction|StopVehicle (LocalVariables|GetAIPawn01Local))
  (Transformation|SetActorLocationAndRotation (LocalVariables|GetPlayerPawnLocal) (Transformation|GetActorLocation (Utilities|Array|Get(acopy) (Variables|/Game/Blueprints/Game/GameInstance01.GameInstance01_C|GetPlayerStarts (LocalVariables|GetGameInstanceLocal)))) (Transformation|GetActorRotation (Utilities|Array|Get(acopy) (Variables|/Game/Blueprints/Game/GameInstance01.GameInstance01_C|GetPlayerStarts (LocalVariables|GetGameInstanceLocal)))) false true)
  (Transformation|SetActorLocationAndRotation (LocalVariables|GetAIPawn01Local) (Transformation|GetActorLocation (Utilities|Array|Get(acopy) (Variables|/Game/Blueprints/Game/GameInstance01.GameInstance01_C|GetPlayerStarts (LocalVariables|GetGameInstanceLocal)) 1)) (Transformation|GetActorRotation (Utilities|Array|Get(acopy) (Variables|/Game/Blueprints/Game/GameInstance01.GameInstance01_C|GetPlayerStarts (LocalVariables|GetGameInstanceLocal)) 1)) false true)
  (Utilities|IsValid (LocalVariables|GetAIPawn02Local)
    (:Is%20Valid
      (CallFunction|StopVehicle (LocalVariables|GetAIPawn02Local))
      (Transformation|SetActorLocationAndRotation (LocalVariables|GetAIPawn02Local) (Transformation|GetActorLocation (Utilities|Array|Get(acopy) (Variables|/Game/Blueprints/Game/GameInstance01.GameInstance01_C|GetPlayerStarts (LocalVariables|GetGameInstanceLocal)) 2)) (Transformation|GetActorRotation (Utilities|Array|Get(acopy) (Variables|/Game/Blueprints/Game/GameInstance01.GameInstance01_C|GetPlayerStarts (LocalVariables|GetGameInstanceLocal)) 2)) false true))
    (:Is%20Not%20Valid
      _))
  (CallFunction|TrackRacesinHeat (LocalVariables|GetGameInstanceLocal))
  (Default|ResetFirstTouchbyPlayer (LocalVariables|GetLevelLogicLocal))
  (Variables|/Game/Blueprints/Player/PlayerControllerSinglePlayer.PlayerControllerSinglePlayer_C|SetVehicleMode (LocalVariables|GetPlayerControllerSinglePlayerLocal) "NewEnumerator0")
  (Variables|/Game/VehicleBP/Sedan/Sedan.Sedan_C|SetTireTemp (LocalVariables|GetPlayerPawnLocal) 0.0))

(fn GetGameInstance
  (bind _asgame_instance_01 (Utilities|Casting|CastToGameInstance01 (Game|GetGameInstance)))
  (return _asgame_instance_01))

(fn SetPlayFabSettings
  (bind _output_get (LocalVariables|SetGameInstanceLocal (CallFunction|GetGameInstance)))
  (Class|PlayFabUtilities|SetPlayFabSettings (.gametitleid (Variables|/Game/Blueprints/Game/GameInstance01.GameInstance01_C|GetPlayFabData _output_get)) (.secretapikey (Variables|/Game/Blueprints/Game/GameInstance01.GameInstance01_C|GetPlayFabData _output_get))))

(fn CreateMainMenu)

(fn LoadPlayFabUserData
  (bind _returnvalue (SaveGame|LoadGamefromSlot "Save02"))
  (Utilities|IsValid _returnvalue
    (:Is%20Valid
      (bind _asplay_fab_user_data_save (Utilities|Casting|CastToPlayFabUserDataSave _returnvalue))
      (Variables|/Game/Blueprints/Game/GameInstance01.GameInstance01_C|SetPlayFabUserData (CallFunction|GetGameInstance) (Variables|/Game/Blueprints/Game/PlayFabUserDataSave.PlayFabUserDataSave_C|GetPlayFabUserData _asplay_fab_user_data_save))
      (return true))
    (:Is%20Not%20Valid
      (return false))))

(fn UpdateRacesWoninHeat
  (params (GameInstance :type Game%20Instance%20Object%20Reference%20%28by%20ref%29) (Place :type Integer))
  (LocalVariables|SetPlaceLocal Place)
  (bind _asgame_instance_01 (Utilities|Casting|CastToGameInstance01 GameInstance))
  (LocalVariables|SetGameInstanceLocal _asgame_instance_01)
  (LocalVariables|SetRacesWonInHeatLocal (Variables|/Game/Blueprints/Game/GameInstance01.GameInstance01_C|GetRacesWonInHeat (LocalVariables|GetGameInstanceLocal)))
  (if (not (Variables|/Game/Blueprints/Game/GameInstance01.GameInstance01_C|GetDisqualified (LocalVariables|GetGameInstanceLocal)))
    (switch int (LocalVariables|GetPlaceLocal)
      (:0
        (bind _output_get (LocalVariables|SetRacesWonInHeatLocal (+ (LocalVariables|GetRacesWonInHeatLocal) 1)))
        (Variables|/Game/Blueprints/Game/GameInstance01.GameInstance01_C|SetRacesWonInHeat (LocalVariables|GetGameInstanceLocal) _output_get)
        (if (== (LocalVariables|GetRacesWonInHeatLocal) 3)
          (LocalVariables|SetWon3InHeatLocal true)
          (return (LocalVariables|GetWon3InHeatLocal)))))))

(fn SingleorMultiplayer
  (bind _returnvalue (Game|GetGameMode))
  (bind _returnvalue_2 (Utilities|GetClass _returnvalue))
  (Utilities|IsValid _returnvalue
    (:Is%20Valid
      (if (== _returnvalue_2 (Variables|/Game/Blueprints/Game/GameInstance01.GameInstance01_C|GetSinglePlayerGameMode (CallFunction|GetGameInstance)))
        (LocalVariables|SetGameMode "NewEnumerator0")
        (return (LocalVariables|GetGameMode))
        (elif (== _returnvalue_2 (Variables|/Game/Blueprints/Game/GameInstance01.GameInstance01_C|GetMultiplayerGameMode (CallFunction|GetGameInstance)))
          (LocalVariables|SetGameMode "NewEnumerator1")
          (return (LocalVariables|GetGameMode))
          (else
            (Development|PrintString 0 "Couldn't determine game mode. Defaulted to SinglePlayer" true true "(R=0.000000,G=0.660000,B=1.000000,A=1.000000)" 2e+01)))))
    (:Is%20Not%20Valid
      (LocalVariables|SetGameMode "NewEnumerator2")
      (return (LocalVariables|GetGameMode)))))

(fn UnstopVehicle
  (params (Pawn :type Sedan%20Object%20Reference))
  (bind _output_get (LocalVariables|SetPawnLocal Pawn))
  (bind _asaicontroller_01 (Utilities|Casting|CastToAIController01 (Pawn|GetController _output_get))
    (:then
      (Default|PressThrottle _asaicontroller_01))
    (:CastFailed
      (Input|EnableInput (LocalVariables|GetPawnLocal) 0)))
  (Class|WheeledVehicleMovementComponent|SetHandbrakeInput (Variables|/Script/PhysXVehicles.WheeledVehicle|GetVehicleMovement (LocalVariables|GetPawnLocal)) false))