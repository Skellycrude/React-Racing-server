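; Multiplayer game mode that obtains a PlayFab title entity when play begins.
; BeginPlay applies PlayFab settings, then requests an entity token with success and failure callbacks.
; Success stores the returned entity as TitleEntity on the game instance, and both outcomes print an on-screen status message.
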(event Custom|CustomEvent_0
  (params (result :type Authentication%20Get%20Entity%20Token%20Response%20Structure) (customData :type Object%20Object%20Reference))
  (Development|PrintString "Get title entity success" true true "(R=0.000000,G=0.660000,B=1.000000,A=1.000000)" 2e+01)
  (Variables|/Game/Blueprints/Game/GameInstance01.GameInstance01_C|SetTitleEntity (CallFunction|GetGameInstance01) (.entity result)))

(event Custom|CustomEvent_1
  (params (error :type Play%20Fab%20Error%20Structure) (customData :type Object%20Object%20Reference))
  (Development|PrintString "Get title entity fail" true true "(R=0.000000,G=0.660000,B=1.000000,A=1.000000)" 2e+01))

(event EventBeginPlay
  (CallFunction|SetPlayFabSettings)
  (|GetEntityToken :onSuccess (delegate Custom|CustomEvent_0) :onFailure (delegate Custom|CustomEvent_1)))

(event EventTick
  (params (DeltaSeconds :type Float%20%28single-precision%29))
  (|CallParentFunction DeltaSeconds) ; This node is disabled and will not be called.\nDrag off pins to build functionality.
)

(fn ConstructionScript
  (|CallParentFunction))